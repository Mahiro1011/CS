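; BP_XSkill is an actor that handles the X skill for the 2D action player.
; On BeginPlay it binds its XSkill event to the skill-motion event of the game instance's SkillObject.
; When that fires and the game instance's Skill is 1, it prints "X" and reports success with that kind to the player obtained from SkillObject.
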(event Custom|XSkill
  (bind _asbp_my_game_instance (Utilities|Casting|CastToBP_MyGameInstance (Game|GetGameInstance)))
  (if (== (Variables|/Game/2DAction/Blueprints/Skill/BP_MyGameInstance.BP_MyGameInstance_C|GetSkill _asbp_my_game_instance) 1)
    (Development|PrintString "X")
    (bind _player (Default|GetPlayer (Variables|/Game/2DAction/Blueprints/Skill/BP_MyGameInstance.BP_MyGameInstance_C|GetSkillObject _asbp_my_game_instance)))
    (Default|SkillResult _player true 1)))

(event EventBeginPlay
  (|CallParentFunction)
  (bind _asbp_my_game_instance (Utilities|Casting|CastToBP_MyGameInstance (Game|GetGameInstance)))
  (EventDispatchers|BindEventtoSkillMotion (Variables|/Game/2DAction/Blueprints/Skill/BP_MyGameInstance.BP_MyGameInstance_C|GetSkillObject _asbp_my_game_instance) (delegate Custom|XSkill)))

(event Collision|EventActorBeginOverlap
  (params (OtherActor :type Actor%20Object%20Reference))
  (|CallParentFunction OtherActor) ; このノードは無効になっているため呼び出せません。\n機能をビルドするにはピンをドラッグしてください。
)

(event EventTick
  (params (DeltaSeconds :type Float%20%28single-precision%29))
  (|CallParentFunction DeltaSeconds) ; このノードは無効になっているため呼び出せません。\n機能をビルドするにはピンをドラッグしてください。
)

(fn ConstructionScript
  (|CallParentFunction))