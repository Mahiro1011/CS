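; BPC_MovementDetecter is a component that gives its owner trace-based sensing of walls, cliffs and the player in a 2D action game.
; Wall and cliff checks trace on Visibility: a line along the given direction, and a downward multi-trace at an offset that reports a cliff on no hit.
; Player detection traces on a separate channel and casts the hit to BP_Player_2D.
; Callers drive all checks, which draw one-frame debug lines.
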(event EventBeginPlay)

(event EventTick
  (params (DeltaSeconds :type Float%20%28single-precision%29)))

(fn IsTouchingWall
  (params (Direction :type Vector))
  (bind _returnvalue (Components|GetOwner))
  (bind _returnvalue_2 (Transformation|GetActorLocation _returnvalue))
  (bind _returnvalue_3 (Collision|LineTraceByChannel _returnvalue_2 (+ _returnvalue_2 (* Direction (Variables|Default|GetWallCheckDistance))) "TraceTypeQuery1" false 0 "ForOneFrame" true "(R=0.792824,G=0.284806,B=1.000000,A=1.000000)"))
  (return _returnvalue_3))

(fn IsatCliff
  (params (Direction :type Vector))
  (bind _returnvalue (Components|GetOwner))
  (bind _cliffcheckoffset (Variables|Default|GetCliffCheckOffset))
  (bind _returnvalue_2 (Transformation|GetActorLocation _returnvalue))
  (bind _returnvalue_3 (* Direction _cliffcheckoffset))
  (bind _returnvalue_4 (+ _returnvalue_2 _returnvalue_3))
  (bind _returnvalue_5 (Collision|MultiLineTraceByChannel _returnvalue_4 (- _returnvalue_4 (* "0.000000,0.000000,1.000000" (Variables|Default|GetCliffCheckDepth))) "TraceTypeQuery1" false 0 "ForOneFrame"))
  (return (not _returnvalue_5)))

(fn DetectPlayer(X)
  (params (Direction :type Vector))
  (bind _returnvalue (Components|GetOwner))
  (bind _returnvalue_2 (Transformation|GetActorLocation _returnvalue))
  (bind (_outhit _returnvalue_3) (Collision|LineTraceByChannel _returnvalue_2 (+ _returnvalue_2 (* Direction (Variables|Default|GetDetacePlayerDistance))) "TraceTypeQuery4" false 0 "ForOneFrame" true "(R=0.000000,G=0.092294,B=1.000000,A=1.000000)"))
  (if _returnvalue_3
    (bind _asbp_player_2d (Utilities|Casting|CastToBP_Player_2D (.hitactor _outhit))
      (:then
        (return true _asbp_player_2d))
      (:CastFailed
        (return false 0)))))