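; AC_Sensor is a sight sensor component that detects actors in front of it.
; CheckSensor runs a multi box trace along the component's forward vector over SightLength, then keeps hit actors that pass CanSeeActor.
; CanSeeActor confirms line of sight with a line trace on a second channel, which must hit the target first.
; It returns the visible actors and whether any were found, with one-frame debug drawing on both traces.
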(event EventBeginPlay)

(event EventTick
  (params (DeltaSeconds :type Float%20%28single-precision%29)))

(fn CheckSensor
  (bind _returnvalue (Transformation|GetWorldTransform))
  (bind _sightlength (Variables|Default|GetSightLength))
  (bind _returnactors (LocalVariables|GetReturnActors))
  (bind (_location _rotation) (Math|Transform|BreakTransform _returnvalue))
  (bind _returnvalue_2 (Math|Vector|GetForwardVector _rotation))
  (bind (_start _end) (CallFunction|CalcRay _location _returnvalue_2 _sightlength))
  (bind _outhits (Class|KismetSystemLibrary|BoxTraceMulti _start _end "0, 0, 0" _rotation "TraceTypeQuery4" false 0 "ForOneFrame" true))
  (for _array_element _outhits
    (bind _returnvalue_3 (CallFunction|CanSeeActor (.HitActor (Collision|BreakHitResult _array_element))))
    (if _returnvalue_3
      (Utilities|Array|Add (LocalVariables|GetReturnActors) (.HitActor (Collision|BreakHitResult _array_element)))))
  (return _returnactors (Utilities|Array|IsNotEmpty _returnactors)))

(fn CanSeeActor
  (params (TargetActor :type Actor%20Object%20Reference))
  (bind _outhit (Collision|LineTraceByChannel (Transformation|GetWorldLocation) (Transformation|GetActorLocation TargetActor) "TraceTypeQuery3" false 0 "ForOneFrame"))
  (return (== (.HitActor (Collision|BreakHitResult _outhit)) TargetActor)))