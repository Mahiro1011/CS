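; BP_Enemy is a 2D action enemy that patrols, charges the player and trades damage on contact.
; Patrol uses BPCMovementDetecter to turn at cliffs or walls and spot the player, switching to Chase1 when off cooldown.
; Chase1 launches toward the target's X every tick, also re-setting the EnablePatrol timer each time.
; Hits deal guardable damage; incoming damage consumes guard count or HP, with brief invincibility and destruction at zero HP.
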(event Custom|RecieveDamage
  (params (DamageQuantity :type Integer))
  ;[1 1 1] 被ダメージ処理
  (if (not (Variables|Default|GetInvincible))
    (Variables|Default|SetInvincible true)
    (if (Variables|Default|GetGuardPossibility)
      (if (== (Variables|Default|GetGuardCount) 0)
        (bind _output_get (Variables|Default|SetHP (Math|Integer|Max(Integer) (- (Variables|Default|GetHP) DamageQuantity)) :!label _label))
        (if (== _output_get 0)
          (Development|PrintString "Enemy is killed!!")
          (Actor|DestroyActor) ; 死亡時のモーションを前に加える
          (else
            (Development|PrintString (Utilities|String|ToString(Integer) _output_get))
            (Utilities|FlowControl|Delay 0.2 :!label _label_2) ; ここにダメージを食らった時のモーション(Timeline)を入れる
            (Variables|Default|SetInvincible false)))
        (else
          (bind _result (Math|Integer|DecrementInt (Variables|Default|GetGuardCount))
            (:%20%20
              (Development|PrintString (Utilities|String|ToString(Integer) _result))
              (goto _label_2)))))
      (else
        (goto _label)))))

(event EventBeginPlay)

(event EventTick
  (params (DeltaSeconds :type Float%20%28single-precision%29))
  (switch Utilities|FlowControl|Switch|SwitchonE_EnemyState (Variables|Default|GetCurrentState)
    (:NewEnumerator1
      (CallFunction|UpdatePatrol))
    (:NewEnumerator2
      (CallFunction|UpdateChase1 3e+02 (.x (Transformation|GetActorLocation (Variables|Default|GetTarget)))))))

(event Collision|EventHit
  (params (MyComp :type Primitive%20Component%20Object%20Reference) (Other :type Actor%20Object%20Reference) (OtherComp :type Primitive%20Component%20Object%20Reference) (bSelfMoved :type Boolean) (HitLocation :type Vector :default "0, 0, 0") (HitNormal :type Vector :default "0, 0, 0") (NormalImpulse :type Vector :default "0, 0, 0") (Hit :type Hit%20Result%20Structure%20%28by%20ref%29))
  (bind _asbp_player_2d (Utilities|Casting|CastToBP_Player_2D Other))
  (Utilities|FlowControl|DoOnce false :!label _label
    (:Completed
      (Default|DamagetoPlayer _asbp_player_2d (Variables|Default|GetAtackDamage) self _asbp_player_2d true)
      (Utilities|FlowControl|Delay 0.2)
      (goto _label Reset))))

(fn ConstructionScript)

(fn UpdatePatrol
  (bind _bpc_movementdetecter (Variables|Default|GetBPC_MovementDetecter))
  ;[1 1 1] 移動処理
  (if (or (Default|IsatCliff _bpc_movementdetecter (Variables|Default|GetMoveDirection)) (Default|IsTouchingWall _bpc_movementdetecter (Variables|Default|GetMoveDirection)))
    (Variables|Default|SetMoveDirection (- "" (Variables|Default|GetMoveDirection))))
  (Pawn|Input|AddMovementInput (Variables|Default|GetMoveDirection) 1.0 false)
  (Transformation|SetActorScale3D (Math|Vector|SelectVector "1.000000,1.000000,1.000000" "-1.000000,1.000000,1.000000" (> (.x (Variables|Default|GetMoveDirection)) 0.0)))
  ;[1 1 1] ターゲット検知
  (bind (_newparam _asbp_player_2d) (Default|DetectPlayer(X) (Variables|Default|GetBPC_MovementDetecter) (Variables|Default|GetMoveDirection)))
  (if _newparam
    (Variables|Default|SetTarget _asbp_player_2d)
    (if (Variables|Default|GetChase1Cooldown)
      (Variables|Default|SetChase1Cooldown false)
      (Utilities|Time|SetTimerbyFunctionName 0 "EnableChase1" 1.0)
      (Variables|Default|SetCurrentState "NewEnumerator2")
      (Development|PrintString "SetTimerEnableChase1"))))

(fn UpdateChase1
  (params (Speed :type Float%20%28double-precision%29) (TargetXLocation :type Float%20%28double-precision%29))
  (Character|LaunchCharacter (* (* Speed (Math|Float|Sign(Float) (- TargetXLocation (.x (Transformation|GetActorLocation self))))) "1.000000,0.000000,0.000000") false false)
  (Utilities|Time|SetTimerbyFunctionName 0 "EnablePatrol" (Variables|Default|GetChase1ContinulyTime))
  (Development|PrintString "SetTimerEnablePatrol"))

(fn EnablePatrol
  (Variables|Default|SetCurrentState "NewEnumerator1")
  (Development|PrintString "Patrol"))

(fn EnableChase1
  (Variables|Default|SetChase1Cooldown true)
  (Development|PrintString "EnableChase1"))